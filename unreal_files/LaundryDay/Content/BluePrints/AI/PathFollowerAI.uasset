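; AI controller that walks an AICharacter along a linked chain of path nodes.
; On BeginPlay it caches the pawn and moves it to its DesiredNode.
; Tick polls the move status and, when it differs from DesiredStatus, advances DesiredNode to its NextNode.
; It then targets the NextNode of that updated node, so the move goal sits one node beyond the stored DesiredNode.
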(event `self.ReceiveBeginPlay`
  ;[1 1 1] AI Move to 1st Node
  (bind _asaicharacter (cast `/Game/BluePrints/AI/AICharacter` (`self.K2_GetPawn`))) ; Cast it to our AI Character
  (bind _output_get (set `self.Stored Pawn` _asaicharacter)) ; Store it as an AI
  (`self.MoveToActor` (`/Game/BluePrints/AI/AICharacter.DesiredNode` _output_get) 15.0))

(event `self.ReceiveTick`
  (params (DeltaSeconds :type "Float (single-precision)"))
  (bind _stored_pawn (`self.Stored Pawn`))
  (bind _nextnode (`/Game/BluePrints/AI/AI_Helper/PathNode.NextNode` (`/Game/BluePrints/AI/AICharacter.DesiredNode` _stored_pawn)))
  ;[1 1 1] Move To Other Nodes
  (if (!= (`self.GetMoveStatus`) (`self.Desired Status`))
    (set `/Game/BluePrints/AI/AICharacter.DesiredNode` _nextnode _stored_pawn)
    (`self.MoveToActor` _nextnode 15.0)))

(fn `UserConstructionScript`)