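; Player character Blueprint, apparently a first attempt, that handles basic movement and a double jump.
; Axis inputs move the character along the forward and right vectors of the control rotation.
; A jump counter allows up to two hold-extendable Jump calls, with release stopping the jump.
; Landing stops active movement and resets the counter.
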(event `InputAxis|Forward/Back`
  (params (AxisValue :type "Float (single-precision)"))
  ;[1 1 1] Movement Controls
  ;;[1 1 1] Move
  (`self.AddMovementInput` (`KismetMathLibrary.GetForwardVector` (`self.GetControlRotation`)) AxisValue))

(event `InputAxis|Left/Right`
  (params (AxisValue :type "Float (single-precision)"))
  ;[1 1 1] Movement Controls
  ;;[1 1 1] Move
  (`self.AddMovementInput` (`KismetMathLibrary.GetRightVector` (`self.GetControlRotation`)) AxisValue))

(event `InputAction|Jump`
  (bind _jump_c (`self.Jump C`))
  ;[1 1 1] Movement Controls
  ;;[1 1 1] Double Jump
  (:`Pressed`
    (set `self.JumpMaxHoldTime` 0.5)
    (if (< _jump_c 2)
      (set `self.Jump C` (+ _jump_c 1))
      (`self.Jump`)))
  (:`Released`
    (`self.StopJumping`)))

(event `self.OnLanded`
  (params (Hit :type "HitResult Structure (by ref)"))
  ;[1 1 1] Movement Controls
  ;;[1 1 1] Double Jump
  (`NavMovementComponent.StopActiveMovement` (`self.CharacterMovement`))
  (set `self.Jump C` 0))

(fn `UserConstructionScript`)