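; Player character Blueprint that handles movement, double jump and sprint input.
; Axis inputs move the character along the control rotation's forward and right vectors.
; A counter caps jumps at two, with hold-to-extend height and a sound at world origin, then resets on landing, which also stops active movement.
; Sprint switches max walk speed between sprint and walk values while setting a state flag.
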(event `InputAxis|Up_Down`
  (params (AxisValue :type "Float (single-precision)"))
  ;[1 1 1] Movement
  (`self.AddMovementInput` (`KismetMathLibrary.GetForwardVector` (`self.GetControlRotation`)) AxisValue))

(event `InputAction|Jump`
  (params (Key :type "Key Structure" :default "AnyKey"))
  (bind _jump_c (`self.Jump_C`))
  ;[1 1 1] Actions
  (:`Pressed`
    (set `self.JumpMaxHoldTime` 0.5)
    (if (< _jump_c 2)
      (set `self.Jump_C` (+ _jump_c 1))
      (`self.Jump`)
      (`GameplayStatics.SpawnSoundAtLocation` "/Game/Sounds/Music/jump.jump")))
  (:`Released`
    (`self.StopJumping`)))

(event `InputAxis|Left_Right`
  (params (AxisValue :type "Float (single-precision)"))
  ;[1 1 1] Movement
  (`self.AddMovementInput` (`KismetMathLibrary.GetRightVector` (`self.GetControlRotation`)) AxisValue))

(event `self.OnLanded`
  (params (Hit :type "HitResult Structure (by ref)"))
  ;[1 1 1] Actions
  ;;[1 1 1] Lets you jump again
  (`NavMovementComponent.StopActiveMovement` (`self.CharacterMovement`))
  (set `self.Jump_C` 0))

(event `InputAction|Sprint`
  (params (Key :type "Key Structure" :default "AnyKey"))
  ;[1 1 1] Sprint
  (:`Pressed`
    (set `self.isSprinting` true)
    (set `CharacterMovementComponent.MaxWalkSpeed` (`self.Sprint Speed`) (`self.CharacterMovement`)))
  (:`Released`
    (set `self.isSprinting` false)
    (set `CharacterMovementComponent.MaxWalkSpeed` (`self.Walk Speed`) (`self.CharacterMovement`))))

(fn `UserConstructionScript`)